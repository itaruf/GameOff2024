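; BP_Djami is an NPC that starts a conversation when the player walks up to it.
; Entering its dialogue capsule starts the dialogue owned by its BPCAct1 component, with that component and the player's DialogueSpeakerComponent as speakers.
; Leaving the capsule ends the current dialogue.
; Both overlap events react only to the player character; BeginPlay and Tick are unused.
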(event OnComponentBeginOverlap(DialogueCapsuleComponent)
  (params (OverlappedComponent :type Primitive%20Component%20Object%20Reference) (OtherActor :type Actor%20Object%20Reference) (OtherComp :type Primitive%20Component%20Object%20Reference) (OtherBodyIndex :type Integer) (bFromSweep :type Boolean) (SweepResult :type Hit%20Result%20Structure%20%28by%20ref%29))
  (bind _returnvalue (Class|PlayerCharacterHelpers|GetPlayerCharacterfromPlayerController))
  (bind _bpc_act1 (Variables|Default|GetBPC_Act1))
  (if (== OtherActor _returnvalue)
    (Class|DialogueSpeakerComponent|StartOwnedDialogue _bpc_act1 (Utilities|Array|MakeArray _bpc_act1 (Actor|GetComponentbyClass _returnvalue "/Script/DialogueTreeRuntime.DialogueSpeakerComponent")) false)))

(event OnComponentEndOverlap(DialogueCapsuleComponent)
  (params (OverlappedComponent :type Primitive%20Component%20Object%20Reference) (OtherActor :type Actor%20Object%20Reference) (OtherComp :type Primitive%20Component%20Object%20Reference) (OtherBodyIndex :type Integer))
  (if (== OtherActor (Class|PlayerCharacterHelpers|GetPlayerCharacterfromPlayerController))
    (Class|DialogueSpeakerComponent|EndCurrentDialogue (Variables|Default|GetBPC_Act1))))

(event EventBeginPlay)

(event Collision|EventActorBeginOverlap
  (params (OtherActor :type Actor%20Object%20Reference)))

(event EventTick
  (params (DeltaSeconds :type Float%20%28single-precision%29)))

(fn ConstructionScript)