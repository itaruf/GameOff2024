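; Player controller that handles interact and skip-dialogue input and controls the player during dialogue and gathering.
; On possess it caches the character and inventory component, then binds events to the dialogue component's start/end and the interact component's gather start/end dispatchers.
; Handlers toggle jumping and move/look input and add or remove the default and dialogue mapping contexts.
; The IgnorePause parameter is unused, and disconnected save, quest and inventory test nodes remain.
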(event Custom|Event%20Enable%20Movement
  ;[1 1 1] Event Enable Movement
  (Class|GameOff2024Character|SetCanJumpDuringDialogue (Variables|Player|GetPlayerCharacter) true)
  (CallFunction|ToggleControls (CallFunction|GetPlayerController) false false false))

(event Custom|Event%20Block%20Movement
  ;[1 1 1] Event Block Movement
  (if (not (Variables|/Game/Dialogues/Components/BP_DialogueComponent.BP_DialogueComponent_C|GetbInDialogue (CallFunction|GetPlayerDialogueComponent)))
    (Class|GameOff2024Character|SetCanJumpDuringDialogue (Variables|Player|GetPlayerCharacter) false)
    (CallFunction|ToggleControls (CallFunction|GetPlayerController) true true true)))

(event Custom|Event%20Gather%20Start
  (Class|GameOff2024Character|SetCanJumpDuringDialogue (Variables|Player|GetPlayerCharacter) false)
  (CallFunction|ToggleControls (CallFunction|GetPlayerController) true false false))

(event Custom|Event%20Gather%20End
  (Class|GameOff2024Character|SetCanJumpDuringDialogue (Variables|Player|GetPlayerCharacter) true)
  (CallFunction|ToggleControls (CallFunction|GetPlayerController) false false false))

(event Custom|Event%20Disable%20Dialogue%20Mapping
  (Input|RemoveMappingContext (PlayerController|LocalPlayerSubsystems|GetEnhancedInputLocalPlayerSubsystem) "/Game/ThirdPerson/Input/IMC_Dialogue.IMC_Dialogue" "(bIgnoreAllPressedKeysUntilRelease=True,bForceImmediately=False,bNotifyUserSettings=False)"))

(event Custom|Event%20Enable%20Dialogue%20Mapping
  (Input|AddMappingContext (PlayerController|LocalPlayerSubsystems|GetEnhancedInputLocalPlayerSubsystem) "/Game/ThirdPerson/Input/IMC_Dialogue.IMC_Dialogue" 0 "(bIgnoreAllPressedKeysUntilRelease=True,bForceImmediately=False,bNotifyUserSettings=False)"))

(event Custom|Event%20Enable%20Default%20Mapping
  (Input|AddMappingContext (PlayerController|LocalPlayerSubsystems|GetEnhancedInputLocalPlayerSubsystem) "/Game/ThirdPerson/Input/IMC_Default.IMC_Default" 1 "(bIgnoreAllPressedKeysUntilRelease=True,bForceImmediately=False,bNotifyUserSettings=False)"))

(event Custom|Event%20Disable%20Default%20Mapping
  (Input|RemoveMappingContext (PlayerController|LocalPlayerSubsystems|GetEnhancedInputLocalPlayerSubsystem) "/Game/ThirdPerson/Input/IMC_Default.IMC_Default" "(bIgnoreAllPressedKeysUntilRelease=True,bForceImmediately=False,bNotifyUserSettings=False)"))

(event Input|EnhancedActionEvents|EnhancedInputActionIA_Interact
  (params (ActionValue :type Boolean) (ElapsedSeconds :type Float%20%28double-precision%29) (TriggeredSeconds :type Float%20%28double-precision%29) (InputAction :type Input%20Action%20Object%20Reference :default "/Game/ThirdPerson/Input/Actions/IA_Interact.IA_Interact"))
  ;[1 1 1] Input Action Interact
  (:Started
    (if (not (Variables|/Game/Dialogues/Components/BP_DialogueComponent.BP_DialogueComponent_C|GetbInDialogue (CallFunction|GetPlayerDialogueComponent)))
      (Default|Interact (Variables|/Game/ThirdPerson/Blueprints/BP_ThirdPersonCharacter.BP_ThirdPersonCharacter_C|GetAC_InteractComponent (Variables|Player|GetPlayerCharacter))))))

(event Input|EnhancedActionEvents|EnhancedInputActionIA_SkipDialogue
  (params (ActionValue :type Boolean) (ElapsedSeconds :type Float%20%28double-precision%29) (TriggeredSeconds :type Float%20%28double-precision%29) (InputAction :type Input%20Action%20Object%20Reference :default "/Game/ThirdPerson/Input/Actions/IA_SkipDialogue.IA_SkipDialogue"))
  ;[1 1 1] Input Action Skip Dialogue
  (:Started
    (bind _returnvalue (Class|DialogueProvider|GetDialogueSpeakerComponent(Message) (Variables|Player|GetPlayerCharacter)))
    (Class|DialogueSpeakerComponent|TrySkipSpeech _returnvalue)))

(event EventBeginPlay
  (Variables|Settings|SetUserSettings (Class|EnhancedInputSubsystemInterface|GetUserSettings (PlayerController|LocalPlayerSubsystems|GetEnhancedInputLocalPlayerSubsystem))))

(event EventPossess
  (params (PossessedPawn :type Pawn%20Object%20Reference))
  (bind _bp_playerdialoguecontroller (CallFunction|GetPlayerDialogueComponent))
  (bind _bp_playerdialoguecontroller_2 (CallFunction|GetPlayerDialogueComponent))
  ;[1 1 1] Event On Possess
  (bind _asbp_third_person_character (Utilities|Casting|CastToBP_ThirdPersonCharacter PossessedPawn))
  (bind _output_get (Variables|Player|SetPlayerCharacter _asbp_third_person_character))
  (bind _inventorycomponent (Class|BPIInventoryProvider|GetInventoryComponent(Message) _output_get))
  (Variables|Default|SetInventoryComponent _inventorycomponent)
  (Utilities|FlowControl|Sequence
    (:then_0
      (EventDispatchers|BindEventtoEDIonDialogueStart (CallFunction|GetPlayerDialogueComponent) (EventDispatchers|CreateEvent :!event StopMovement)))
    (:then_1
      (EventDispatchers|BindEventtoEDIonDialogueStart _bp_playerdialoguecontroller_2 (EventDispatchers|CreateEvent :!event Custom|Event%20Block%20Movement))
      (EventDispatchers|BindEventtoEDIonDialogueStart _bp_playerdialoguecontroller_2 (EventDispatchers|CreateEvent :!event Custom|Event%20Enable%20Dialogue%20Mapping))
      (EventDispatchers|BindEventtoEDIonDialogueStart _bp_playerdialoguecontroller_2 (EventDispatchers|CreateEvent :!event Custom|Event%20Disable%20Default%20Mapping)))
    (:then_2
      (EventDispatchers|BindEventtoEDIonGatherStart (Variables|/Game/ThirdPerson/Blueprints/BP_ThirdPersonCharacter.BP_ThirdPersonCharacter_C|GetAC_InteractComponent (Variables|Player|GetPlayerCharacter)) (EventDispatchers|CreateEvent :!event Custom|Event%20Gather%20Start))
      (EventDispatchers|BindEventtoEDIonGatherEnd (Variables|/Game/ThirdPerson/Blueprints/BP_ThirdPersonCharacter.BP_ThirdPersonCharacter_C|GetAC_InteractComponent (Variables|Player|GetPlayerCharacter)) (EventDispatchers|CreateEvent :!event Custom|Event%20Gather%20End)))
    (:then_3
      (EventDispatchers|AssignEDIonDialogueEnd _bp_playerdialoguecontroller (EventDispatchers|CreateEvent :!event Custom|Event%20Enable%20Movement))
      (EventDispatchers|AssignEDIonDialogueEnd _bp_playerdialoguecontroller (EventDispatchers|CreateEvent :!event Custom|Event%20Enable%20Default%20Mapping))
      (EventDispatchers|AssignEDIonDialogueEnd _bp_playerdialoguecontroller (EventDispatchers|CreateEvent :!event Custom|Event%20Disable%20Dialogue%20Mapping)))))

(event Input|KeyboardEvents|F
  (params (Key :type Key%20Structure :default "None")))

(event Input|KeyboardEvents|R
  (params (Key :type Key%20Structure :default "None")))

(event Input|KeyboardEvents|I
  (params (Key :type Key%20Structure :default "None")))

(event Input|KeyboardEvents|J
  (params (Key :type Key%20Structure :default "None")))

(event Input|KeyboardEvents|O
  (params (Key :type Key%20Structure :default "None")))

(event Input|KeyboardEvents|T
  (params (Key :type Key%20Structure :default "None")))

(event Input|KeyboardEvents|U
  (params (Key :type Key%20Structure :default "None")))

(event Input|KeyboardEvents|M
  (params (Key :type Key%20Structure :default "None")))

(event Input|KeyboardEvents|V
  (params (Key :type Key%20Structure :default "None")))

(event Input|KeyboardEvents|K
  (params (Key :type Key%20Structure :default "None")))

(event Input|KeyboardEvents|P
  (params (Key :type Key%20Structure :default "None")))

(fn ConstructionScript)

(fn ToggleControls
  (params (bIgnoreMove? :type Boolean) (bIgnoreLook? :type Boolean) (bIgnorePause? :type Boolean))
  (Input|SetIgnoreMoveInput bIgnoreMove?)
  (Input|SetIgnoreLookInput bIgnoreLook?))

(fn GetPlayerCharacter
  (return (Variables|Player|GetPlayerCharacter)))

(fn SetPlayerCharacter
  (params (NewPlayerCharacter :type BP%20Third%20Person%20Character%20Object%20Reference))
  (Variables|Player|SetPlayerCharacter NewPlayerCharacter))