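; Player interaction component that finds a nearby NPC in front of the player and starts its dialogue.
; SphereTraceForInteractables overlaps Pawns around the player, picks the one closest to the capsule's forward direction within MaxAngle, and starts that BP_NPC's current dialogue.
; A line trace to the target only prints its result, without gating dialogue.
; The camera-based TraceForInteractables is unused, and BeginPlay's looping timer has no event bound.
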(event Custom|SphereTraceForInteractables
  (bind _player (Variables|Default|GetPlayer))
  (bind _returnvalue (Transformation|GetActorLocation _player))
  (Rendering|Debug|DrawDebugSphere _returnvalue (Variables|Default|GetSphereRadius) 12 "(R=1.000000,G=1.000000,B=1.000000,A=1.000000)" 3.0 1.0)
  (bind (_outactors _returnvalue_2) (Collision|SphereOverlapActors _returnvalue (Variables|Default|GetSphereRadius) (Utilities|Array|MakeArray "ObjectTypeQuery3") 0 (Utilities|Array|MakeArray (Variables|Default|GetPlayer))))
  (if _returnvalue_2
    (Variables|Default|SetClosestActor 0)
    (Variables|Default|SetBestAngle 3.6e+02)
    (Variables|Default|SetAngleDegrees 0.0)
    (Variables|Default|SetDot 0.0)
    (for _array_element _outactors
      (bind _output_get (Variables|Default|SetDirectionToActor (Math|Vector|Normalize (- (Transformation|GetActorLocation _array_element) _returnvalue))))
      (bind _output_get_2 (Variables|Default|SetDot (Math|Vector|DotProduct _output_get (Math|Vector|GetForwardVector (Variables|/Script/Engine.Character|GetCapsuleComponent _player)))))
      (bind _output_get_3 (Variables|Default|SetAngleDegrees (Math|Trig|RadiansToDegrees (Math|Trig|Acos(Degrees) _output_get_2))))
      (if (and (< _output_get_3 (Variables|Default|GetMaxAngle)) (< _output_get_3 (Variables|Default|GetBestAngle)))
        (Variables|Default|SetClosestActor _array_element)
        (Variables|Default|SetBestAngle (Variables|Default|GetAngleDegrees))))
    (Development|PrintString (Utilities|GetDisplayName (Variables|Default|GetClosestActor)))
    (Development|PrintString "End")
    (bind _outhit (Collision|LineTraceByChannel (Transformation|GetActorLocation (Variables|Default|GetPlayer)) (Transformation|GetActorLocation (Variables|Default|GetClosestActor)) "TraceTypeQuery2" true (Utilities|Array|MakeArray (Variables|Default|GetPlayer)) "ForDuration"))
    (Development|PrintString (Utilities|String|ToString(Boolean) (== (.hitactor _outhit) (Variables|Default|GetClosestActor))))
    (bind _asbp_npc (Utilities|Casting|CastToBP_NPC (Variables|Default|GetClosestActor)))
    (Class|DialogueSpeakerComponent|StartDialogue (Variables|/Game/Characters/NPC/BP_NPC.BP_NPC_C|GetBP_NPCDialogueComponent _asbp_npc) (.Value (Utilities|Map|Find (Variables|/Game/Dialogues/Components/BP_NPCDialogueComponent.BP_NPCDialogueComponent_C|GetDialogues (Variables|/Game/Characters/NPC/BP_NPC.BP_NPC_C|GetBP_NPCDialogueComponent _asbp_npc)) (Variables|/Game/Dialogues/Components/BP_NPCDialogueComponent.BP_NPCDialogueComponent_C|GetCurrentKey (Variables|/Game/Characters/NPC/BP_NPC.BP_NPC_C|GetBP_NPCDialogueComponent _asbp_npc)))) (Utilities|Array|MakeArray (Variables|/Game/Characters/NPC/BP_NPC.BP_NPC_C|GetBP_NPCDialogueComponent _asbp_npc) (Variables|/Game/ThirdPerson/Blueprints/BP_ThirdPersonCharacter.BP_ThirdPersonCharacter_C|GetBP_PlayerDialogueComponent (Variables|Default|GetPlayer))) false)
    (else
      (Development|PrintString "No Overlapped Actors"))))

(event EventBeginPlay
  (Utilities|FlowControl|Sequence
    (:then_0
      (bind _asbp_third_person_character (Utilities|Casting|CastToBP_ThirdPersonCharacter (Components|GetOwner)))
      (Variables|Default|SetPlayer _asbp_third_person_character))
    (:then_1
      (bind _returnvalue (Utilities|Time|SetTimerbyEvent 0 (Utilities|Time|GetWorldDeltaSeconds) true))
      (Variables|Default|SetTraceForInteractablesHandle _returnvalue))))

(event EventTick
  (params (DeltaSeconds :type Float%20%28single-precision%29)))

(fn TraceforInteractables
  (bind _bp_player_controller (CallFunction|GetPlayerController))
  (bind _location (Pawn|GetPlayerViewPoint _bp_player_controller))
  (bind _outhit (Collision|LineTraceByChannel _location (+ _location (* (Default|GetCameraForward _bp_player_controller) (Variables|Default|GetTraceForInteractablesRange))) "TraceTypeQuery2" false (Utilities|Array|MakeArray (Variables|Default|GetPlayer)) "ForOneFrame"))
  (return _outhit))