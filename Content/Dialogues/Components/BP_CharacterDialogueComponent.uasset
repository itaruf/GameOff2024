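; Character dialogue component that stores a character's dialogues in a keyed map and starts them by key.
; StartDialogueByKey looks up the dialogue and passes it with the supplied speakers to StartDialogue, with resume off and no check for a missing key.
; Separate setters store the current key and current dialogue; starting by key does not update either.
; BeginPlay only calls the parent, and Tick is disabled.
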(event EventBeginPlay
  (|CallParentFunction))

(event EventTick
  (params (DeltaSeconds :type Float%20%28single-precision%29))
  (|CallParentFunction DeltaSeconds) ; This node is disabled and will not be called.\nDrag off pins to build functionality.
)

(fn GetDialoguebyKey
  (params (Key :type Name))
  (return (.Value (Utilities|Map|Find (Variables|Dialogues|GetDialogues) Key))))

(fn StartDialoguebyKey
  (params (Key :type Name) (InSpeakers :type Array%20of%20Dialogue%20Speaker%20Component%20Object%20References))
  (Class|DialogueSpeakerComponent|StartDialogue (CallFunction|GetDialoguebyKey Key) InSpeakers false))

(fn SetCurrentKey
  (params (NewKey :type Name))
  (Variables|Default|SetCurrentKey NewKey))

(fn SetCurrentDialogue
  (params (NewDialogue :type Dialogue%20Object%20Reference))
  (Variables|Default|SetCurrentDialogue NewDialogue))