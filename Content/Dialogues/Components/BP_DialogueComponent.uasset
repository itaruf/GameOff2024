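; Dialogue speaker component that holds a keyed map of dialogues for its owning actor and starts the current one on interaction.
; On BeginPlay it registers the owner and dialogue keys with the game instance, caches the owned dialogue and binds to a dialogue-change event.
; Interaction pairs the initiator's speaker component with itself as speakers.
; Helpers start dialogues by key or switch the current and owned dialogue.
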(event Custom|On%20Interacted
  (params (Initiator :type Actor%20Object%20Reference))
  (bind _currentdialogue (Variables|Default|GetCurrentDialogue))
  (if (Utilities|Map|IsNotEmpty (Variables|Dialogues|GetDialogues))
    (bind _returnvalue (Class|DialogueProvider|GetDialogueSpeakerComponent(Message) Initiator))
    (Utilities|IsValid _currentdialogue
      (:Is%20Valid
        (Class|DialogueSpeakerComponent|StartDialogue _currentdialogue (Utilities|Array|MakeArray _returnvalue self) false)))))

(event EventBeginPlay
  (|CallParentFunction)
  (Utilities|FlowControl|Sequence
    (:then_0
      (bind _keys (Utilities|Map|Keys (Variables|Dialogues|GetDialogues)))
      (Default|RegisterDialogues (CallFunction|GetGameInstance) (Components|GetOwner) _keys))
    (:then_1
      (Variables|Default|SetCurrentDialogue (Class|DialogueSpeakerComponent|GetOwnedDialogue)))
    (:then_2
      (EventDispatchers|BindEventtoEDIonDialogueChange (EventDispatchers|CreateEvent :!event UpdateDialogue)))))

(fn GetDialoguebyKey
  (params (Key :type Name))
  (return (.Value (Utilities|Map|Find (Variables|Dialogues|GetDialogues) Key))))

(fn StartDialoguebyKey
  (params (Key :type Name) (InSpeakers :type Array%20of%20Dialogue%20Speaker%20Component%20Object%20References))
  (Class|DialogueSpeakerComponent|StartDialogue (CallFunction|GetDialoguebyKey Key) InSpeakers false))

(fn SetCurrentKey
  (params (NewKey :type Name))
  (Variables|Default|SetCurrentKey NewKey))

(fn SetCurrentDialogue
  (params (NewDialogue :type Dialogue%20Object%20Reference))
  (Variables|Default|SetCurrentDialogue NewDialogue))

(fn UpdateDialogue
  (params (NewKey :type Name))
  (CallFunction|SetCurrentKey NewKey)
  (CallFunction|SetCurrentDialogue (CallFunction|GetDialoguebyKey (Variables|Default|GetCurrentKey)))
  (Class|DialogueSpeakerComponent|SetOwnedDialogue (Variables|Default|GetCurrentDialogue)))