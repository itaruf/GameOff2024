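; Player dialogue component that locks player controls while a dialogue is running.
; On BeginPlay it caches the player character and binds handlers to the dialogue start and end events of the player dialogue component.
; The start handler ignores move, look and pause input through the player controller, guarded by an InDialogue flag against repeat calls.
; The end handler restores all three and clears the flag.
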(event Custom|Custom%20Event%20%20Dialogue%20End
  (Default|ToggleControls (CallFunction|GetPlayerController) false false false)
  (Variables|Default|SetbInDialogue false))

(event Custom|Custom%20Event%20Dialogue%20Start
  (if (not (Variables|Default|GetbInDialogue))
    (Default|ToggleControls (CallFunction|GetPlayerController) true true true)
    (Variables|Default|SetbInDialogue true)))

(event EventBeginPlay
  (bind _bp_playerdialoguecontroller (CallFunction|GetPlayerDialogueComponent))
  (|CallParentFunction)
  (Utilities|FlowControl|Sequence
    (:then_0
      (Variables|Default|SetPlayerCharacter (CallFunction|GetPlayerCharacterfromPlayerController)))
    (:then_1
      (EventDispatchers|BindEventtoEDIonDialogueStart _bp_playerdialoguecontroller (EventDispatchers|CreateEvent :!event Custom|Custom%20Event%20Dialogue%20Start)))
    (:then_2
      (EventDispatchers|BindEventtoEDIonDialogueEnd _bp_playerdialoguecontroller (EventDispatchers|CreateEvent :!event Custom|Custom%20Event%20%20Dialogue%20End)))))