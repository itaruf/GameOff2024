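; Inventory actor component that stores items in a key-to-item map and handles adding, querying and removing stacks.
; Adds take a struct or data table row, merging existing entries with stacks clamped to their maximum.
; Removals fire event dispatchers, though RemoveItemStackByKey writes partial removals back unchanged and fires none.
; A separate Inventory map serves slot lookups by index, and the BeginPlay dispatcher bindings are disconnected.
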(event EventBeginPlay)

(fn GetInventoryComponent
  (return self))

(fn AddItem
  (params (InventoryItem :type F%20Inventory%20Item%20Structure))
  (bind _data (Utilities|Struct|BreakF_InventoryItem InventoryItem))
  (bind _items (Variables|Default|GetItems))
  (bind (_key _stack) (Utilities|Struct|BreakF_ItemData _data))
  (bind (_value _returnvalue) (Utilities|Map|Find _items _key))
  (bind (_key_2 _type _name _icon _description _stack_2 _itemtemplate) (Utilities|Struct|BreakF_ItemData (.data _value)))
  ;[1 1 1] Does it exist ?
  (if _returnvalue
    (Utilities|Map|Add (Variables|Default|GetItems) _key_2 (Utilities|Struct|MakeF_InventoryItem (.guid _value) (.maxquantity _value) (.isstackable? _value) (Utilities|Struct|MakeF_ItemData _key_2 _type _name _icon _description (Math|Integer|Clamp(Integer) (+ _stack_2 _stack) 0 (.maxquantity _value)) _itemtemplate)))
    (else
      ;[1 1 1] Add as a new entry
      (Utilities|Map|Add (Variables|Default|GetItems) _key InventoryItem))))

(fn AddItemfromDataTable
  (params (InventoryItem :type Data%20Table%20Row%20Handle%20Structure) (Stack :type Integer))
  (bind (_datatable _rowname) (Utilities|Struct|BreakDataTableRowHandle InventoryItem))
  (bind _items (Variables|Default|GetItems))
  (bind (_value _returnvalue) (Utilities|Map|Find _items _rowname))
  (bind (_key _type _name _icon _description _stack _itemtemplate) (Utilities|Struct|BreakF_ItemData (.data _value)))
  (bind _returnvalue_2 (Utilities|GetDataTableRow _datatable _rowname)
    (:then
      ;[1 1 1] Does it exist ?
      (if _returnvalue
        (Utilities|Map|Add (Variables|Default|GetItems) _key (Utilities|Struct|MakeF_InventoryItem (.guid _value) (.maxquantity _value) (.isstackable? _value) (Utilities|Struct|MakeF_ItemData _key _type _name _icon _description (Math|Integer|Clamp(Integer) (+ _stack Stack) 0 (.maxquantity _value)) _itemtemplate)))
        (else
          ;[1 1 1] Add as a new entry
          (Utilities|Map|Add (Variables|Default|GetItems) _rowname _returnvalue_2))))))

(fn GetItembyKey
  (params (Key :type Name))
  (bind _items (Variables|Default|GetItems))
  (bind (_value _returnvalue) (Utilities|Map|Find _items Key))
  (return _value _returnvalue))

(fn HasItem?
  (params (Key :type Name))
  (return (Utilities|Map|Contains (Variables|Default|GetItems) Key)))

(fn HasEnoughItemStack?
  (params (Key :type Name) (Stack :type Integer))
  (bind (_inventoryitem _found_) (Inventory|GetItembyKey Key))
  (if _found_
    (return (>= (Utilities|Struct|BreakF_ItemData (Utilities|Struct|BreakF_InventoryItem _inventoryitem)) Stack))
    (else
      (return false))))

(fn HasItemStack
  (params (DT_InventoryItem :type Data%20Table%20Row%20Handle%20Structure) (StackNumber :type Integer) (ComparisonSymbol :type E_MathSymbol%20Enum :default "NewEnumerator0"))
  (bind _key (Inventory|GetInventoryItemKeyfromDataTable DT_InventoryItem))
  (bind (_stack _found_) (Inventory|GetItemStackbyKey _key))
  (if _found_
    (bind _boolean (CallFunction|CompareValues _stack StackNumber ComparisonSymbol))
    (return _boolean)
    (else
      (return false))))

(fn GetItemStackbyKey
  (params (Key :type Name))
  (bind (_inventoryitem _found_) (Inventory|GetItembyKey Key))
  (if _found_
    (return (Utilities|Struct|BreakF_ItemData (Utilities|Struct|BreakF_InventoryItem _inventoryitem)) true)
    (else
      (return -1 false))))

(fn RemoveItembyKey
  (params (Key :type Name))
  (bind _returnvalue (Utilities|Map|Remove (Variables|Default|GetItems) Key))
  (if _returnvalue
    (Default|CallEDIonItemRemoved Key)))

(fn RemoveItemStackbyKey
  (params (Key :type Name) (StackToRemove :type Integer))
  (bind (_inventoryitem _found_) (Inventory|GetItembyKey Key))
  (bind (_guid _maxquantity _isstackable_ _data) (Utilities|Struct|BreakF_InventoryItem _inventoryitem))
  (bind (_key _type _name _icon _description _stack) (Utilities|Struct|BreakF_ItemData _data))
  (if _found_
    ;[1 1 1] Check if the number of stack is > 0
    (if (> (Math|Integer|Clamp(Integer) (- _stack StackToRemove) 0 _maxquantity) 0)
      (Utilities|Map|Add (Variables|Default|GetItems) _key _inventoryitem)
      (else
        ;[1 1 1] If the stack is 0, remove the item
        (Inventory|RemoveItembyKey _key)))))

(fn DebugItemRemovedbyKey
  (params (Key :type Name))
  (Development|PrintString (Utilities|String|Append (Utilities|String|ToString(Name) Key) ":  removed completely")))

(fn DebugItemStackRemovedbyKey
  (params (Key :type Name) (Stack :type Integer))
  (Development|PrintString (Utilities|String|Append (Utilities|String|ToString(Name) Key) " - stack: " (Utilities|String|ToString(Integer) Stack) " removed")))

(fn GetInventorySlot
  (params (Index :type Integer))
  (bind _inventory (Variables|Default|GetInventory))
  (bind (_value _returnvalue) (Utilities|Map|Find _inventory Index))
  (return _value _returnvalue))

(fn RemoveItemStackfromDataTable
  (params (DT_InventoryItem :type Data%20Table%20Row%20Handle%20Structure) (NumberStack :type Integer))
  (bind (_inventoryitem _found) (CallFunction|GetDefaultInventoryItemfromDataTable DT_InventoryItem))
  (bind _items (Variables|Default|GetItems))
  (bind _data (Utilities|Struct|BreakF_InventoryItem _inventoryitem))
  (bind _key (Utilities|Struct|BreakF_ItemData _data))
  (bind _value (Utilities|Map|Find _items _key))
  (if _found
    (if (>= NumberStack (.stack (.data _value)))
      (Inventory|RemoveItembyKey (.key (.data _value)))
      (else
        (Utilities|Map|Add (Variables|Default|GetItems) (.key (.data _value)) (Utilities|Struct|MakeF_InventoryItem (.guid _value) (.maxquantity _value) (.isstackable? _value) (Utilities|Struct|MakeF_ItemData (.key (.data _value)) (.type (.data _value)) (.name (.data _value)) (.icon (.data _value)) (.description (.data _value)) (- (.stack (.data _value)) NumberStack) (.itemtemplate (.data _value)))))
        (Default|CallEDIonItemStackRemoved (.key (.data _value)) NumberStack)))))

(fn GetInventoryItemKeyfromDataTable
  (params (InventoryItem :type Data%20Table%20Row%20Handle%20Structure))
  (return (.rowname InventoryItem)))