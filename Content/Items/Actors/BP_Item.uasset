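; BP_Item is a world pickup actor that carries inventory item data and is collected when it collides with the player.
; On BeginPlay it binds the EDIOnItemPickedUp dispatcher, then copies item data from the InventoryItemTemplate class defaults unless OverrideTemplate is set.
; A static mesh hit prints a debug string; if the player character caused it, the item broadcasts its data through that dispatcher and destroys itself.
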(event OnComponentHit(StaticMesh)
  (params (HitComponent :type Primitive%20Component%20Object%20Reference) (OtherActor :type Actor%20Object%20Reference) (OtherComp :type Primitive%20Component%20Object%20Reference) (NormalImpulse :type Vector :default "0, 0, 0") (Hit :type Hit%20Result%20Structure%20%28by%20ref%29))
  (Development|PrintString "Hello")
  (if (== OtherActor (Class|PlayerCharacterHelpers|GetPlayerCharacterfromPlayerController))
    (Default|CallEDIonItemPickedUp (Variables|OverrideTemplate|GetInventoryItemData))
    (Actor|DestroyActor)))

(event EventBeginPlay
  (Utilities|FlowControl|Sequence
    (:then_0
      (EventDispatchers|BindEventtoEDIonItemPickedUp (EventDispatchers|CreateEvent (CallFunction|GetPlayerInventoryComponent) :!event TransformItemtoInventoryItem)))
    (:then_1
      (CallFunction|InitItemData))))

(fn ConstructionScript)

(fn SetItemData
  (params (NewData :type F%20Item%20Data%20Structure))
  (Variables|OverrideTemplate|SetInventoryItemData (Utilities|Struct|MakeF_ItemData (.type NewData) (.id NewData) (.name NewData) (.icon NewData) (.description NewData) (.stack NewData) (.stackmax NewData) (.itemtemplate NewData))))

(fn InitItemData
  (if (not (Variables|OverrideTemplate|GetbOverrideTemplate?))
    (CallFunction|SetItemData (Utilities|GetClassDefaults (Variables|Data|Template|GetInventoryItemTemplate)))))