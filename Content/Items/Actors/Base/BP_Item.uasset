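; Base world item actor that can be picked up or, when not itemizable, passes interaction to its dialogue component.
; On BeginPlay it binds the item-picked-up dispatcher and builds its inventory data from a data table row, unless the template is overridden.
; Interacting with an itemizable item broadcasts that data through the dispatcher and destroys the actor.
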(event EventBeginPlay
  (Utilities|FlowControl|Sequence
    (:then_0
      (EventDispatchers|BindEventtoEDIonItemPickedUp (EventDispatchers|CreateEvent (CallFunction|GetPlayerInventoryComponent) :!event AddItem)))
    (:then_1
      (CallFunction|InitItemData))))

(event EventInteract
  (params (Initiator :type Actor%20Object%20Reference) (Interactee :type Actor%20Object%20Reference))
  (if (Variables|InventoryItem|GetbItemizable)
    (Default|CallEDIonItemPickedUp (Variables|InventoryItem|GetInventoryItemData))
    (Actor|DestroyActor)
    (else
      (Default|OnInteracted (Variables|Default|GetBP_DialogueComponent) Initiator))))

(fn ConstructionScript)

(fn SetItemData
  (params (NewData :type F%20Inventory%20Item%20Structure))
  (Variables|InventoryItem|SetInventoryItemData NewData))

(fn InitItemData
  (bind _dtinventorydata (Variables|InventoryItem|GetDTInventoryData))
  (if (not (Variables|OverrideTemplate|GetbOverrideTemplate?))
    (Utilities|IsValid (.datatable _dtinventorydata)
      (:Is%20Valid
        (bind _returnvalue (Utilities|GetDataTableRow (.datatable _dtinventorydata) (.rowname _dtinventorydata))
          (:then
            (CallFunction|SetItemData (Utilities|Struct|MakeF_InventoryItem (.Guid (Utilities|Struct|BreakF_InventoryItem _returnvalue)) (.MaxQuantity (Utilities|Struct|BreakF_InventoryItem _returnvalue)) (.IsStackable? (Utilities|Struct|BreakF_InventoryItem _returnvalue)) (.Data (Utilities|Struct|BreakF_InventoryItem _returnvalue))))))))))

(fn GetCollisionObjectType
  (return (Collision|GetCollisionObjectType (Variables|Default|GetStaticMesh))))